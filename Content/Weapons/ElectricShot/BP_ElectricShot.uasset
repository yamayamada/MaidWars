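; BP_ElectricShot is a projectile actor for the electric shot weapon that damages another BP_Owner on contact.
; On BeginPlay it caches the Aura component's forward vector, then moves along it each Tick by Speed, scaled by delta time, without sweeping.
; When its Sphere overlaps a BP_Owner other than FireOwner, it asks FireOwner to send fixed damage to that target and destroys itself.
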(event OnComponentBeginOverlap(Sphere)
  (params (OverlappedComponent :type Primitive%20Component%20Object%20Reference) (OtherActor :type Actor%20Object%20Reference) (OtherComp :type Primitive%20Component%20Object%20Reference) (OtherBodyIndex :type Integer) (bFromSweep :type Boolean) (SweepResult :type Hit%20Result%20Structure%20%28by%20ref%29))
  (bind _fireowner (Variables|Default|GetFireOwner))
  (bind _asbp_owner (Utilities|Casting|CastToBP_Owner OtherActor))
  (if (not (== _asbp_owner _fireowner))
    (Default|SendDamage _fireowner _asbp_owner 1e+01)
    (Actor|DestroyActor)))

(event EventBeginPlay
  (Variables|Default|Setmove (Math|Vector|GetForwardVector (Variables|Default|GetAura))))

(event Collision|EventActorBeginOverlap
  (params (OtherActor :type Actor%20Object%20Reference)))

(event EventTick
  (params (DeltaSeconds :type Float%20%28single-precision%29))
  (Transformation|SetActorLocation (+ (Transformation|GetActorLocation) (* (* (Variables|Default|Getmove) (Variables|Default|GetSpeed)) (/ DeltaSeconds 0.01))) false false))

(fn ConstructionScript)