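; BP_Bomb is a thrown bomb projectile that flies in an arc and spawns BP_Blast when it detonates.
; BeginPlay takes a horizontal direction from the Arrow, then Tick advances it by Speed per frame, unscaled by delta time.
; A time-based sine offset shapes the height while the actor spins.
; It explodes when height drops to a fixed threshold or its Sphere overlaps a BP_Owner other than FireOwner.
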(event OnComponentBeginOverlap(Sphere)
  (params (OverlappedComponent :type Primitive%20Component%20Object%20Reference) (OtherActor :type Actor%20Object%20Reference) (OtherComp :type Primitive%20Component%20Object%20Reference) (OtherBodyIndex :type Integer) (bFromSweep :type Boolean) (SweepResult :type Hit%20Result%20Structure%20%28by%20ref%29))
  (bind _asbp_owner (Utilities|Casting|CastToBP_Owner OtherActor))
  (if (!= _asbp_owner (Variables|Default|GetFireOwner))
    (Game|SpawnActorfromClass "/Game/Weapons/Bomb/BP_Blast.BP_Blast_C" (Math|Transform|MakeTransform (Transformation|GetActorLocation) "0, 0, 0" "1,1,1") "Undefined" 0 0)
    (Actor|DestroyActor)))

(event EventBeginPlay
  (bind _arrow (Variables|Default|GetArrow))
  (bind _returnvalue (Math|Vector|GetForwardVector _arrow))
  (Variables|Default|SetMove (Math|Vector|MakeVector (.x _returnvalue) (.y _returnvalue) 0.0))
  (Variables|Default|SetLocation (Transformation|GetActorLocation)))

(event Collision|EventActorBeginOverlap
  (params (OtherActor :type Actor%20Object%20Reference)))

(event EventTick
  (params (DeltaSeconds :type Float%20%28single-precision%29))
  (Variables|Default|SetTime (+ DeltaSeconds (Variables|Default|GetTime)))
  (Variables|Default|SetLocation (+ (Variables|Default|GetLocation) (* (Variables|Default|GetMove) (Variables|Default|GetSpeed))))
  (if (<= (+ (.z (Variables|Default|GetLocation)) (* (Variables|Default|GetHigh) (Math|Trig|Sin(Degrees) (* (/ (Variables|Default|GetTime) (Variables|Default|GetMaxTime)) 1.8e+02)))) -5.0)
    (Game|SpawnActorfromClass "/Game/Weapons/Bomb/BP_Blast.BP_Blast_C" (Math|Transform|MakeTransform (Transformation|GetActorLocation) "0, 0, 0" "1,1,1") "Undefined" 0 0)
    (Actor|DestroyActor)
    (else
      (Transformation|SetActorLocation (Math|Vector|MakeVector (.x (Variables|Default|GetLocation)) (.y (Variables|Default|GetLocation)) (+ (.z (Variables|Default|GetLocation)) (* (Variables|Default|GetHigh) (Math|Trig|Sin(Degrees) (* (/ (Variables|Default|GetTime) (Variables|Default|GetMaxTime)) 1.8e+02))))) false false)
      (Transformation|AddLocalRotation (Variables|Default|GetDefaultSceneRoot) "-10.000000,0.000000,0.000000" false false))))

(fn ConstructionScript)