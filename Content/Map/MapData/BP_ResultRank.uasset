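; BP_ResultRank is a map actor that grows vertically to a height set by a rank, apparently for a results display.
; SetStart picks a target Z scale from the rank, with higher placings growing taller, and starts the animation.
; Tick raises the root's Z scale at a frame-rate-compensated speed until it reaches that target, then stops.
; Reset, also run on BeginPlay, restores unit scale and clears the state.
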(event Custom|Reset
  (Transformation|SetWorldScale3D (Variables|Default|GetDefaultSceneRoot) "1.000000,1.000000,1.000000")
  (Variables|Default|SetisStart false)
  (Variables|Default|SetisEnd false)
  (Variables|Default|SetScale_Z 1.0))

(event EventBeginPlay
  (Transformation|SetWorldScale3D (Variables|Default|GetDefaultSceneRoot) "1.000000,1.000000,1.000000")
  (Variables|Default|SetisStart false)
  (Variables|Default|SetisEnd false)
  (Variables|Default|SetScale_Z 1.0))

(event Collision|EventActorBeginOverlap
  (params (OtherActor :type Actor%20Object%20Reference)))

(event EventTick
  (params (DeltaSeconds :type Float%20%28single-precision%29))
  (if (and (Variables|Default|GetisStart) (not (Variables|Default|GetisEnd)))
    (Variables|Default|SetFrameFit (/ DeltaSeconds 0.01))
    (bind _output_get (Variables|Default|SetScale_Z (+ (Variables|Default|GetScale_Z) (* (Variables|Default|GetFrameFit) 0.04))))
    (if (>= _output_get (Variables|Default|GetTargetScale))
      (Transformation|SetWorldScale3D (Variables|Default|GetDefaultSceneRoot) (Math|Vector|MakeVector 1.0 1.0 (Variables|Default|GetTargetScale)))
      (Variables|Default|SetisEnd true)
      (else
        (Transformation|SetWorldScale3D (Variables|Default|GetDefaultSceneRoot) (Math|Vector|MakeVector 1.0 1.0 (Variables|Default|GetScale_Z)))))))

(fn ConstructionScript)

(fn SetStart
  (params (rank :type Integer))
  (switch int rank
    (:Default
      _)
    (:0
      _)
    (:1
      (Variables|Default|SetTargetScale 2.0))
    (:2
      (Variables|Default|SetTargetScale 1.6))
    (:3
      (Variables|Default|SetTargetScale 1.3))
    (:4
      (Variables|Default|SetTargetScale 1.0)))
  (Variables|Default|SetisStart true))