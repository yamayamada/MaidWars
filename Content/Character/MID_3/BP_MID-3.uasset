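; BP_MID-3 is a playable character Blueprint with four input-driven attacks and cosmetic booster effects, extending a parent class's BeginPlay and Tick.
; Each attack input checks CanAttack, then sets status through AttackOption and picks a bullet class: electric shot, missile, bomb or laser.
; The special attack also shows and animates a laser beam component.
; Two socket-attached booster emitters are toggled from Tick by StickDown, using paired DoOnce gates to act only on changes.
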(event EventBeginPlay
  (|CallParentFunction)
  (CallFunction|BoosterSet))

(event EventTick
  (params (DeltaSeconds :type Float%20%28single-precision%29))
  (|CallParentFunction DeltaSeconds)
  (CallFunction|BoosterManagement))

(event Input|ActionEvents|InputActionSpecialAttack
  (params (Key :type Key%20Structure))
  ;[1 1 1] Attack
  (:Pressed
    (if (.AttackOK? (CallFunction|CanAttack))
      (CallFunction|AttackOption "NewEnumerator6" 0.0 0.0 true)
      (Variables|Default|SetMyBullet "/Game/Weapons/Laser/BP_Laser.BP_Laser_C")
      (CallFunction|LaserBeamStart))))

(event Input|ActionEvents|InputActionUniqueAttack
  (params (Key :type Key%20Structure))
  ;[1 1 1] Attack
  (:Pressed
    (if (.AttackOK? (CallFunction|CanAttack))
      (CallFunction|AttackOption "NewEnumerator5" 0.0 0.0 true)
      (Variables|Default|SetMyBullet "/Game/Weapons/Bomb/BP_Bomb.BP_Bomb_C"))))

(event Input|ActionEvents|InputActionFirstAttack
  (params (Key :type Key%20Structure))
  ;[1 1 1] Attack
  (:Pressed
    (CallFunction|AttackContinuou)
    (if (.AttackOK? (CallFunction|CanAttack))
      (CallFunction|AttackOption "NewEnumerator1" 0.0 6e+02 true)
      (Variables|Default|SetMyBullet "/Game/Weapons/ElectricShot/BP_ElectricShot.BP_ElectricShot_C"))))

(event Input|ActionEvents|InputActionSecondAttack
  (params (Key :type Key%20Structure))
  ;[1 1 1] Attack
  (:Pressed
    (if (.AttackOK? (CallFunction|CanAttack))
      (CallFunction|AttackOption "NewEnumerator3" 0.0 6e+02 true)
      (Variables|Default|SetMyBullet "/Game/Weapons/Missile/BP_Missile.BP_Missile_C"))))

(fn ConstructionScript
  (|CallParentFunction))

(fn BoosterSet
  (bind _returnvalue (Effects|SpawnEmitterAttached "/Game/Effect/Particle/P_Booster.P_Booster" (Variables|Character|GetMesh) "Booster_1"))
  (bind _returnvalue_2 (Effects|SpawnEmitterAttached "/Game/Effect/Particle/P_Booster.P_Booster" (Variables|Character|GetMesh) "Booster_2"))
  (Variables|Default|SetBoosters (Utilities|Array|MakeArray _returnvalue _returnvalue_2)))

(fn BoosterManagement
  (if (Variables|Default|GetStickDown?)
    (Utilities|FlowControl|DoOnce false :!label _label
      (:Completed
        (for _array_element (Variables|Default|GetBoosters)
          (Rendering|SetVisibility _array_element true false)
          (goto _label_2 Reset))))
    (else
      (Utilities|FlowControl|DoOnce false :!label _label_2
        (:Completed
          (for _array_element_2 (Variables|Default|GetBoosters)
            (Rendering|SetVisibility _array_element_2 false false)
            (goto _label Reset)))))))

(fn LaserBeamStart
  (bind _laserbeam1 (Variables|Default|GetLaserBeam1))
  (Rendering|SetVisibility _laserbeam1 true false)
  (Components|Animation|PlayAnimation _laserbeam1 "/Game/Weapons/Laser/LaserBeam/Chariot_LaserBeam.Chariot_LaserBeam" false))

(fn LaserBeamEnd
  (Components|Animation|PlayAnimation (Variables|Default|GetLaserBeam1) "/Game/Weapons/Laser/LaserBeam/Chariot_LaserBeamOver.Chariot_LaserBeamOver" false))