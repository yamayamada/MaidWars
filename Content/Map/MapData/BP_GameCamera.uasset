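; Map game camera that turns to face a target actor, both in the construction script and on BeginPlay.
; BeginPlay also caches the camera's base transform and the high and low BP_MapSizeTarget locations.
; SetPlayer keeps the joined players for helpers computing their average XY position and X spread.
; The movement and spread-based pitch nodes using these helpers are unwired, Tick is empty, and GetHorizontal is an unfinished stub.
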(event EventBeginPlay
  (Transformation|SetActorRotation (Math|Rotator|FindLookatRotation (Transformation|GetActorLocation) (Transformation|GetActorLocation (Variables|Default|GetTargetActor))))
  (Variables|Default|SetBaseTramsform (Transformation|GetWorldTransform (Variables|CameraActor|GetCameraComponent)))
  (bind _outactors (Actor|GetAllActorsOfClass "/Game/Map/MapData/BP_MapSizeTarget.BP_MapSizeTarget_C"))
  (Utilities|IsValid (Utilities|Array|Get(acopy) _outactors)
    (:Is%20Valid
      (if (Variables|/Game/Map/MapData/BP_MapSizeTarget.BP_MapSizeTarget_C|GetisHigh (Utilities|Array|Get(acopy) _outactors))
        (Variables|Default|SetTargetLocation_high (Transformation|GetActorLocation (Utilities|Array|Get(acopy) _outactors)))
        (Variables|Default|SetTargetLocation_low (Transformation|GetActorLocation (Utilities|Array|Get(acopy) _outactors 1)))
        (else
          (Variables|Default|SetTargetLocation_high (Transformation|GetActorLocation (Utilities|Array|Get(acopy) _outactors 1)))
          (Variables|Default|SetTargetLocation_low (Transformation|GetActorLocation (Utilities|Array|Get(acopy) _outactors))))))
    (:Is%20Not%20Valid
      (Development|PrintString "NOACTOR"))))

(event Collision|EventActorBeginOverlap
  (params (OtherActor :type Actor%20Object%20Reference)))

(event EventTick
  (params (DeltaSeconds :type Float%20%28single-precision%29)))

(fn ConstructionScript
  (Transformation|SetActorRotation (Math|Rotator|FindLookatRotation (Transformation|GetActorLocation) (Transformation|GetActorLocation (Variables|Default|GetTargetActor)))))

(fn SetPlayer
  (params (AllPlayer :type Array%20of%20BP%20Owner%20Object%20References))
  (bind _player (Variables|Default|GetPlayer))
  (Variables|Default|Setflg true)
  (Utilities|Array|Clear _player)
  (for _array_element AllPlayer
    (if (Variables|/Game/Character/BP_Owner.BP_Owner_C|GetIsJoin _array_element)
      (Utilities|Array|Add _player _array_element))))

(fn GetVertical
  (if (Variables|Default|Getflg)
    (for (_array_element _array_index) (Variables|Default|GetPlayer)
      (if (== _array_index 0)
        (LocalVariables|SetHigh (.x (Transformation|GetActorLocation _array_element)))
        (LocalVariables|SetLow (.x (Transformation|GetActorLocation _array_element)))
        (elif (> (.x (Transformation|GetActorLocation _array_element)) (LocalVariables|GetHigh))
          (LocalVariables|SetHigh (.x (Transformation|GetActorLocation _array_element)))
          (elif (< (.x (Transformation|GetActorLocation _array_element)) (LocalVariables|GetLow))
            (LocalVariables|SetLow (.x (Transformation|GetActorLocation _array_element)))))))
    (return (- (LocalVariables|GetHigh) (LocalVariables|GetLow)))))

(fn GetHorizontal
  (for (_array_element _array_index) (Variables|Default|GetPlayer)
    (if (not (== _array_index 0))
      (if (not (> (.y (Transformation|GetActorLocation _array_element)) 0.0))
        (if (< (.y (Transformation|GetActorLocation _array_element)) 0.0)
          _)))))

(fn GetPlayerCenter
  (if (Variables|Default|Getflg)
    (for _array_element (Variables|Default|GetPlayer)
      (LocalVariables|Setvec (+ (Math|Vector2D|MakeVector2D (.x (Transformation|GetActorLocation _array_element)) (.y (Transformation|GetActorLocation _array_element))) (LocalVariables|Getvec))))
    (return (Math|Vector|MakeVector (.x (/ (LocalVariables|Getvec) (Math|Conversions|ToFloat(Integer) (Utilities|Array|Length (Variables|Default|GetPlayer))))) (.y (/ (LocalVariables|Getvec) (Math|Conversions|ToFloat(Integer) (Utilities|Array|Length (Variables|Default|GetPlayer))))) (.z (.location (Variables|Default|GetBaseTramsform)))))))