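; BP_Mid3 is a player character Blueprint that maps four attack inputs (first, second, special, unique) to attacks.
; Each input calls AttackContinuou and AttackJudge, then sets PlayerStatus and passes attack power and move speed to AttackSetting.
; Special and unique attacks proceed only when AttackJudge is false, while first and second proceed either way.
; The second attack also triggers LongDistanceAttack, and BeginPlay clears MyBullet after the parent's setup.
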(event EventBeginPlay
  (|CallParentFunction)
  (Variables|Default|SetMyBullet 0))

(event EventTick
  (params (DeltaSeconds :type Float%20%28single-precision%29))
  (|CallParentFunction DeltaSeconds) ; This node is disabled and will not be called.\nDrag off pins to build functionality.
)

(event Input|ActionEvents|InputActionSpecialAttack
  (params (Key :type Key%20Structure))
  ;[1 1 1] Attack
  (:Pressed
    (CallFunction|AttackContinuou)
    (if (not (CallFunction|AttackJudge))
      (Variables|Default|SetPlayerStatus "NewEnumerator6")
      (CallFunction|AttackSetting 1e+01 0.0))))

(event Input|ActionEvents|InputActionUniqueAttack
  (params (Key :type Key%20Structure))
  ;[1 1 1] Attack
  (:Pressed
    (CallFunction|AttackContinuou)
    (if (not (CallFunction|AttackJudge))
      (Variables|Default|SetPlayerStatus "NewEnumerator5")
      (CallFunction|AttackSetting 1e+02 0.0))))

(event Input|ActionEvents|InputActionFirstAttack
  (params (Key :type Key%20Structure))
  ;[1 1 1] Attack
  (:Pressed
    (CallFunction|AttackContinuou)
    (if (CallFunction|AttackJudge)
      _
      (else
        _))
    (Variables|Default|SetPlayerStatus "NewEnumerator1")
    (CallFunction|AttackSetting 1e+01 1e+02)))

(event Input|ActionEvents|InputActionSecondAttack
  (params (Key :type Key%20Structure))
  ;[1 1 1] Attack
  (:Pressed
    (CallFunction|AttackContinuou)
    (if (CallFunction|AttackJudge)
      _
      (else
        _))
    (Variables|Default|SetPlayerStatus "NewEnumerator3")
    (CallFunction|AttackSetting 2e+01 6e+02)
    (CallFunction|LongDistanceAttack)))

(fn ConstructionScript
  (|CallParentFunction))