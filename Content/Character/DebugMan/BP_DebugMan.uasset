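; DebugMan is a playable character Blueprint with four input-driven attacks and a booster particle attached to its mesh at BeginPlay.
; Each attack input calls inherited-style helpers, with attacks setting a player status plus power and move speed, and the second adding a long-distance attack.
; Tick enables Sword or Leg collision from that status, and their overlaps pass the hit actor to HitActorDuplication.
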(event OnComponentBeginOverlap(Sword)
  (params (OverlappedComponent :type Primitive%20Component%20Object%20Reference) (OtherActor :type Actor%20Object%20Reference) (OtherComp :type Primitive%20Component%20Object%20Reference) (OtherBodyIndex :type Integer) (bFromSweep :type Boolean) (SweepResult :type Hit%20Result%20Structure%20%28by%20ref%29))
  (CallFunction|HitActorDuplication OtherActor))

(event OnComponentBeginOverlap(Leg)
  (params (OverlappedComponent :type Primitive%20Component%20Object%20Reference) (OtherActor :type Actor%20Object%20Reference) (OtherComp :type Primitive%20Component%20Object%20Reference) (OtherBodyIndex :type Integer) (bFromSweep :type Boolean) (SweepResult :type Hit%20Result%20Structure%20%28by%20ref%29))
  (CallFunction|HitActorDuplication OtherActor))

(event EventBeginPlay
  (|CallParentFunction)
  (Variables|Default|SetMyBullet 0)
  (CallFunction|BoosterON))

(event EventTick
  (params (DeltaSeconds :type Float%20%28single-precision%29))
  (bind _playerstatus (Variables|Default|GetPlayerStatus))
  (|CallParentFunction DeltaSeconds)
  (CallFunction|CollisionSetting (Variables|Default|GetSword) (Math|Boolean|ORBoolean (Utilities|Enum|Equal(Enum) _playerstatus "NewEnumerator1") (Utilities|Enum|Equal(Enum) _playerstatus "NewEnumerator3") (Utilities|Enum|Equal(Enum) _playerstatus "NewEnumerator6")))
  (CallFunction|CollisionSetting (Variables|Default|GetLeg) (Utilities|Enum|Equal(Enum) (Variables|Default|GetPlayerStatus) "NewEnumerator5")))

(event Input|ActionEvents|InputActionSpecialAttack
  (params (Key :type Key%20Structure))
  ;[1 1 1] Attack
  (:Pressed
    (CallFunction|AttackContinuou)
    (if (not (CallFunction|AttackJudge))
      (Variables|Default|SetPlayerStatus "NewEnumerator6")
      (CallFunction|AttackSetting 1e+01 0.0))))

(event Input|ActionEvents|InputActionUniqueAttack
  (params (Key :type Key%20Structure))
  ;[1 1 1] Attack
  (:Pressed
    (CallFunction|AttackContinuou)
    (if (not (CallFunction|AttackJudge))
      (Variables|Default|SetPlayerStatus "NewEnumerator5")
      (CallFunction|AttackSetting 1e+02 0.0))))

(event Input|ActionEvents|InputActionFirstAttack
  (params (Key :type Key%20Structure))
  ;[1 1 1] Attack
  (:Pressed
    (CallFunction|AttackContinuou)
    (if (CallFunction|AttackJudge)
      _
      (else
        _))
    (Variables|Default|SetPlayerStatus "NewEnumerator1")
    (CallFunction|AttackSetting 1e+01 1e+02)))

(event Input|ActionEvents|InputActionSecondAttack
  (params (Key :type Key%20Structure))
  ;[1 1 1] Attack
  (:Pressed
    (CallFunction|AttackContinuou)
    (if (CallFunction|AttackJudge)
      _
      (else
        _))
    (Variables|Default|SetPlayerStatus "NewEnumerator3")
    (CallFunction|AttackSetting 2e+01 6e+02)
    (CallFunction|LongDistanceAttack)))

(fn ConstructionScript
  (|CallParentFunction))

(fn BoosterON
  (Effects|SpawnEmitterAttached "/Game/Effect/Particle/P_Booster.P_Booster" (Variables|Character|GetMesh) "BoosterSocket" "0, 0, 0" "0, 0, 0" "1.000000,1.000000,1.000000" "SnapToTarget"))