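; BP_Missile is a projectile that flies in a straight line and notifies the BP_Owner actor it hits.
; BeginPlay stores the Arrow's forward vector as its direction and attaches a booster particle effect.
; Tick moves it without sweep, scaled by delta time, while speed grows by a fixed step every frame.
; Capsule overlap with a BP_Owner other than FireOwner calls SendDamage with zero base damage, then destroys the missile.
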(event OnComponentBeginOverlap(Capsule)
  (params (OverlappedComponent :type Primitive%20Component%20Object%20Reference) (OtherActor :type Actor%20Object%20Reference) (OtherComp :type Primitive%20Component%20Object%20Reference) (OtherBodyIndex :type Integer) (bFromSweep :type Boolean) (SweepResult :type Hit%20Result%20Structure%20%28by%20ref%29))
  (bind _asbp_owner (Utilities|Casting|CastToBP_Owner OtherActor))
  (if (not (== _asbp_owner (Variables|Default|GetFireOwner)))
    (Default|SendDamage _asbp_owner 0 0.0)
    (Actor|DestroyActor)))

(event EventBeginPlay
  (Variables|Default|SetMove (Math|Vector|GetForwardVector (Variables|Default|GetArrow)))
  (Effects|SpawnEmitterAttached "/Game/Effect/Particle/P_Booster.P_Booster" (Variables|Default|GetMissile) "None" "0, 0, 0" "0.000000, 0,-90.000000"))

(event Collision|EventActorBeginOverlap
  (params (OtherActor :type Actor%20Object%20Reference)))

(event EventTick
  (params (DeltaSeconds :type Float%20%28single-precision%29))
  (Transformation|SetActorLocation (+ (Transformation|GetActorLocation) (* (* (Variables|Default|GetMove) (Variables|Default|GetSpeed)) (/ DeltaSeconds 0.01))) false false)
  (Variables|Default|SetSpeed (+ (Variables|Default|GetSpeed) 0.15)))

(fn ConstructionScript)