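; Base player character for a combat game, with gated world-axis movement, health, attacks and material skin cycling.
; Attack helpers set status, power and walk speed, deal damage to other BP_Owner actors with duplicate-hit tracking, or spawn owned projectiles.
; Damage is ignored during the hit-reaction status, otherwise playing a montage or triggering death.
; Death launches the character randomly without collision, then notifies BP_MaidGameInstance and moves it to a spawn point.
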(event Custom|DestroyPlayerMove
  ;[1 1 1] 死亡処理
  (Utilities|FlowControl|Delay 1.0)
  (Collision|SetCollisionEnabled (Variables|Character|GetMesh) "QueryAndPhysics")
  (Collision|SetCollisionEnabled (Variables|Collision|GetCapsuleComponent) "QueryAndPhysics")
  (Variables|/Script/Engine.MovementComponent|SetVelocity (Variables|Character|GetCharacterMovement) "0, 0, 0")
  (bind _asbp_maid_game_instance (Utilities|Casting|CastToBP_MaidGameInstance (Game|GetGameInstance)))
  (Default|SetDeadPlayer _asbp_maid_game_instance self)
  (Transformation|SetActorLocation (Default|GetSpawnPoint _asbp_maid_game_instance "NewEnumerator0" (.AsPlayer%20Controller (Utilities|Casting|CastToPlayerController (Pawn|GetController)))) false false))

(event EventBeginPlay
  (CallFunction|Initialize))

(event EventTick
  (params (DeltaSeconds :type Float%20%28single-precision%29)))

(event Game|Damage|EventAnyDamage
  (params (Damage :type Float%20%28single-precision%29) (DamageType :type Damage%20Type%20Object%20Reference) (InstigatedBy :type Controller%20Object%20Reference) (DamageCauser :type Actor%20Object%20Reference))
  ;[1 1 1] Damage
  (if (not (Utilities|Enum|Equal(Enum) (Variables|Default|GetPlayerStatus) "NewEnumerator8"))
    (CallFunction|ReceiveDamage Damage)))

(event Input|AxisEvents|InputAxisMoveForward
  (params (AxisValue :type Float%20%28single-precision%29))
  ;[1 1 1] Move
  (if (CallFunction|CanMove)
    (Pawn|Input|AddMovementInput "1.000000, 0, 0" AxisValue false)
    (bind (_stickdown_ _stickdirection) (CallFunction|GetLeftStickDirection AxisValue (stale Input|AxisEvents|InputAxisMoveRight AxisValue)))
    (bind _output_get (Variables|Default|SetStickDown? _stickdown_))
    (if _output_get
      (Variables|Default|SetLeftDerection _stickdirection)
      (else
        (Variables|Default|SetLeftDerection (Transformation|GetActorForwardVector self))))))

(event Input|AxisEvents|InputAxisMoveRight
  (params (AxisValue :type Float%20%28single-precision%29))
  ;[1 1 1] Move
  (if (CallFunction|CanMove)
    (Pawn|Input|AddMovementInput "0,1.000000, 0" AxisValue false)
    (bind (_stickdown_ _stickdirection) (CallFunction|GetLeftStickDirection (stale Input|AxisEvents|InputAxisMoveForward AxisValue) AxisValue))
    (bind _output_get (Variables|Default|SetStickDown? _stickdown_))
    (if _output_get
      (Variables|Default|SetLeftDerection _stickdirection)
      (else
        (Variables|Default|SetLeftDerection (Transformation|GetActorForwardVector self))))))

(fn ConstructionScript)

(fn CanMove
  (return (and (not (Variables|Default|GetIsDead)) (Variables|Default|GetIsGame))))

(fn GetLeftStickDirection
  (params (Xinput :type Float%20%28single-precision%29) (Yinput :type Float%20%28single-precision%29))
  (bind _returnvalue (Pawn|GetControlRotation :!class /Script/Engine.Pawn))
  (bind _yaw (Math|Rotator|BreakRotator _returnvalue))
  (bind _returnvalue_2 (Math|Rotator|MakeRotator 0.0 0.0 _yaw))
  (bind _returnvalue_3 (Math|Vector|GetForwardVector _returnvalue_2))
  (bind _returnvalue_4 (Math|Vector|GetRightVector _returnvalue_2))
  (bind _returnvalue_5 (* _returnvalue_3 Xinput))
  (bind _returnvalue_6 (* _returnvalue_4 Yinput))
  (bind _returnvalue_7 (+ _returnvalue_5 _returnvalue_6))
  (return (>= (Math|Vector|VectorLength _returnvalue_7) 0.5) _returnvalue_7))

(fn AttackSetting
  (params (AttackPower :type Float%20%28single-precision%29) (MoveSpeed :type Float%20%28single-precision%29))
  (Variables|Default|SetAttackPower AttackPower)
  (Variables|/Script/Engine.CharacterMovementComponent|SetMaxWalkSpeed (Variables|Character|GetCharacterMovement) MoveSpeed))

(fn CanAttack
  (bind _self self)
  (bind _returnvalue (Transformation|GetVelocity _self))
  (bind _returnvalue_2 (Math|Vector|VectorLength _returnvalue))
  (bind _returnvalue_3 (> _returnvalue_2 0.0))
  (if (Math|Boolean|ANDBoolean (Utilities|Enum|Equal(Enum) (Variables|Default|GetPlayerStatus) "NewEnumerator0") (not (Variables|Default|GetIsAttackTiming)) (Variables|Default|GetIsGame))
    (return true _returnvalue_3)
    (else
      (return false _returnvalue_3))))

(fn HitActorDuplication
  (params (Object :type Object%20Object%20Reference))
  (bind _asbp_owner (Utilities|Casting|CastToBP_Owner Object))
  (Variables|Default|SetHitActor _asbp_owner)
  (for _array_element (Variables|Default|GetAttackHitActor)
    (Variables|Default|SetAttackHit (== _array_element (Variables|Default|GetHitActor))))
  (if (and (!= _asbp_owner self) (not (Variables|Default|GetAttackHit)))
    (CallFunction|SendDamage (Variables|Default|GetHitActor) (Variables|Default|GetAttackPower))
    (Utilities|Array|Add (Variables|Default|GetAttackHitActor) (Variables|Default|GetHitActor))
    (Effects|SpawnEmitteratLocation "/Game/Effect/Particle/P_Hit.P_Hit" (Transformation|GetActorLocation (Variables|Default|GetHitActor)))))

(fn CollisionSetting
  (params (Target :type Primitive%20Component%20Object%20Reference) (CollisionON :type Boolean))
  (if (and CollisionON (Variables|Default|GetCollisionOn))
    (Utilities|FlowControl|DoOnce false :!label _label
      (:Completed
        (Collision|SetCollisionEnabled Target "QueryAndPhysics")
        (goto _label_2 Reset)))
    (else
      (Utilities|FlowControl|DoOnce false :!label _label_2
        (:Completed
          (Collision|SetCollisionEnabled Target "NoCollision")
          (goto _label Reset))))))

(fn ReceiveDamage
  (params (Damage :type Float%20%28single-precision%29))
  (bind _output_get (Variables|Default|SetLife (- (Variables|Default|GetLife) Damage)))
  (if (<= _output_get 0.0)
    (CallFunction|PlayerDead)
    (else
      (Variables|Default|SetPlayerStatus "NewEnumerator8")
      (Animation|PlayAnimMontage "/Game/Character/MID_3/Animation/Damage.Damage" 0.95 "None"))))

(fn SendDamage
  (params (DamagedActor :type Actor%20Object%20Reference) (BaseDamage :type Float%20%28single-precision%29))
  (Game|Damage|ApplyDamage DamagedActor BaseDamage 0 0))

(fn PlayerDead
  (Variables|Default|SetPlayerStatus "NewEnumerator9")
  (Character|LaunchCharacter (Math|Vector|MakeVector (Math|Random|RandomFloatinRange -1e+04 1e+04) (Math|Random|RandomFloatinRange -1e+04 1e+04) 2e+02) false false)
  (Utilities|FlowControl|DoOnce false
    (:Completed
      (Collision|SetCollisionEnabled (Variables|Character|GetMesh) "NoCollision")
      (Collision|SetCollisionEnabled (Variables|Collision|GetCapsuleComponent) "NoCollision")
      (CallFunction|DestroyPlayerMove))))

(fn BulletCreate
  (params (SpawnLocation :type Vector))
  (bind _returnvalue (Game|SpawnActorfromClass (Variables|Default|GetMyBullet) (Math|Transform|MakeTransform SpawnLocation (Transformation|GetWorldRotation (Variables|Collision|GetCapsuleComponent))) "Undefined" 0 0))
  (bind _asbp_weapons (Utilities|Casting|CastToBP_Weapons _returnvalue))
  (Default|SetFireOwner _asbp_weapons self))

(fn LongDistanceAttack
  (Variables|/Script/Engine.CharacterMovementComponent|SetbOrientRotationToMovement (Variables|Character|GetCharacterMovement) false))

(fn AttackContinuou
  (if (Variables|Default|GetAnimeLoop?)
    (Variables|Default|SetAttackContinuous true)))

(fn AttackOption
  (params (PlayerStatus :type PlayerState%20Enum :default "NewEnumerator0") (AttackPower :type Float%20%28single-precision%29) (MoveSpeed :type Float%20%28single-precision%29) (DirectionFixed :type Boolean))
  (Variables|Default|SetPlayerStatus PlayerStatus)
  (CallFunction|AttackSetting AttackPower MoveSpeed)
  (Variables|Default|SetIsAttackTiming true)
  (if DirectionFixed
    (CallFunction|LongDistanceAttack)))

(fn Initialize
  (Variables|Default|SetLife (Variables|Default|GetDefaultLife)))

(fn SkinChange
  (params (Dimension%201 :type Integer))
  (bind _mymaterial (Variables|Default|GetMyMaterial))
  (bind _returnvalue (Utilities|Array|Length _mymaterial))
  (bind _output_get (Variables|Default|SetMaterialNumber (+ Dimension%201 (Variables|Default|GetMaterialNumber))))
  (if (< _output_get 0)
    (Variables|Default|SetMaterialNumber (- _returnvalue 1))
    (elif (>= _output_get _returnvalue)
      (Variables|Default|SetMaterialNumber 0)))
  (Rendering|Material|SetMaterial (Variables|Character|GetMesh) 0 (Utilities|Array|Get(acopy) (Variables|Default|GetMyMaterial) (Variables|Default|GetMaterialNumber))))