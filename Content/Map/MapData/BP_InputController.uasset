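; Per-controller menu input actor that drives the HUD flow between Title, Select, Game and Result.
; BeginPlay finds the BP_Owner character sharing its Controller; Tick polls input by HUD mode, using DoOnce gates to edge-detect gamepad presses.
; In Select it toggles join, notifies HUDMain, moves the character between spawn points, cycles a five-value color index, and lets joined players start the game.
; JoinReset resyncs join state and position from the character.
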(event Custom|JoinReset
  (bind _instance (Variables|Default|GetInstance))
  (bind _player (Variables|Default|GetPlayer))
  (bind _controller (Variables|Default|GetController))
  (bind _output_get (Variables|Default|SetisJoin (Variables|/Game/Character/BP_Owner.BP_Owner_C|GetIsJoin (Variables|Default|GetPlayer))))
  (Default|JoinEvent (Variables|Default|GetHUDMain) self _output_get)
  (if _output_get
    (Transformation|SetActorLocation _player (Default|GetSpawnPoint _instance "NewEnumerator2" _controller) false false)
    (else
      (Transformation|SetActorLocation _player (Default|GetSpawnPoint _instance "NewEnumerator0" _controller) false false))))

(event EventBeginPlay
  ;[1 1 1] 保持しているControllerとおなじControllerを持つPlayerCharacterを検索
  (bind _outactors (Actor|GetAllActorsOfClass "/Game/Character/BP_Owner.BP_Owner_C"))
  (for _array_element _outactors
    (if (== (Pawn|GetController _array_element) (Variables|Default|GetController))
      (Variables|Default|SetPlayer _array_element)))
  (bind _asbp_maid_game_instance (Utilities|Casting|CastToBP_MaidGameInstance (Game|GetGameInstance)))
  (Variables|Default|SetInstance _asbp_maid_game_instance))

(event Collision|EventActorBeginOverlap
  (params (OtherActor :type Actor%20Object%20Reference)))

(event EventTick
  (params (DeltaSeconds :type Float%20%28single-precision%29))
  (bind _player (Variables|Default|GetPlayer))
  (bind _instance (Variables|Default|GetInstance))
  (bind _controller (Variables|Default|GetController))
  (switch Utilities|FlowControl|Switch|SwitchonE_HUDMode (Variables|/Game/UI/HUD/HUD_Main.HUD_Main_C|GetthisHUDMode (Variables|Default|GetHUDMain))
    (:NewEnumerator0
      (if (Utilities|AnyKey)
        (Default|ChangeHUD (Variables|Default|GetHUDMain) "NewEnumerator1")))
    (:NewEnumerator1
      (Utilities|FlowControl|Sequence
        (:then_0
          ;[1 1 1] JoinのOnOffの入力を受け付け、HUD_Selectに伝える
          (if (== (Class|PlayerController|GetInputAnalogKeyState (Variables|Default|GetController) "Gamepad_FaceButton_Bottom") 1.0)
            (Utilities|FlowControl|DoOnce false :!label _label
              (:Completed
                (if (not (Variables|Default|GetisJoin))
                  (bind _output_get (Variables|Default|SetisJoin true))
                  (Default|JoinEvent (Variables|Default|GetHUDMain) self _output_get)
                  ;[1 1 1] Joinしたら同じControllerを持つCharacterの位置を変更させる
                  (if (Variables|Default|GetisJoin) :!label _label_2
                    (Transformation|SetActorLocation _player (Default|GetSpawnPoint _instance "NewEnumerator2" _controller) false false)
                    (Variables|/Game/Character/BP_Owner.BP_Owner_C|SetIsJoin _player true)
                    (else
                      (Transformation|SetActorLocation _player (Default|GetSpawnPoint _instance "NewEnumerator0" _controller) false false)
                      (Variables|/Game/Character/BP_Owner.BP_Owner_C|SetIsJoin _player false))))))
            (else
              (goto _label Reset))))
        (:then_1
          (if (== (Class|PlayerController|GetInputAnalogKeyState (Variables|Default|GetController) "Gamepad_FaceButton_Right") 1.0)
            (Utilities|FlowControl|DoOnce false :!label _label_3
              (:Completed
                (if (Variables|Default|GetisJoin)
                  (bind _output_get_2 (Variables|Default|SetisJoin false))
                  (Default|JoinEvent (Variables|Default|GetHUDMain) self _output_get_2)
                  (goto _label_2))))
            (else
              (goto _label_3 Reset))))
        (:then_2
          ;[1 1 1] 左右入力
          (if (>= (Class|PlayerController|GetInputAnalogKeyState (Variables|Default|GetController) "Gamepad_LeftStick_Right") 1.0)
            (Utilities|FlowControl|DoOnce false :!label _label_4
              (:Completed
                (bind _result (Math|Integer|IncrementInt (Variables|Default|Getcolornum))
                  (:%20%20
                    (if (>= _result 5)
                      (Variables|Default|Setcolornum 0))))))
            (else
              (goto _label_4 Reset))))
        (:then_3
          (if (>= (Class|PlayerController|GetInputAnalogKeyState (Variables|Default|GetController) "Gamepad_LeftStick_Left") 1.0)
            (Utilities|FlowControl|DoOnce false :!label _label_5
              (:Completed
                (bind _result_2 (Math|Integer|DecrementInt (Variables|Default|Getcolornum))
                  (:%20%20
                    (if (< _result_2 0)
                      (Variables|Default|Setcolornum 4))))))
            (else
              (goto _label_5 Reset))))
        (:then_4
          ;[1 1 1] 上下入力
          (if (>= (Class|PlayerController|GetInputAnalogKeyState (Variables|Default|GetController) "Gamepad_LeftStick_Up") 1.0)
            (Utilities|FlowControl|DoOnce false :!label _label_6
              (:Completed
                (bind _result_3 (Math|Integer|IncrementInt (Variables|Default|Getcolornum))
                  (:%20%20
                    (if (>= _result_3 5)
                      (Variables|Default|Setcolornum 0))))))
            (else
              (goto _label_6 Reset))))
        (:then_5
          (if (>= (Class|PlayerController|GetInputAnalogKeyState (Variables|Default|GetController) "Gamepad_LeftStick_Down") 1.0)
            (Utilities|FlowControl|DoOnce false :!label _label_7
              (:Completed
                (bind _result_4 (Math|Integer|DecrementInt (Variables|Default|Getcolornum))
                  (:%20%20
                    (if (< _result_4 0)
                      (Variables|Default|Setcolornum 4))))))
            (else
              (goto _label_7 Reset))))
        (:then_6
          ;[1 1 1] GameStart
          (if (== (Class|PlayerController|GetInputAnalogKeyState (Variables|Default|GetController) "Gamepad_Special_Right") 1.0)
            (Utilities|FlowControl|DoOnce false :!label _label_8
              (:Completed
                (if (Variables|Default|GetisJoin)
                  (Default|ChangeHUD (Variables|Default|GetHUDMain) "NewEnumerator2"))))
            (else
              (goto _label_8 Reset))))))
    (:NewEnumerator3
      (if (Utilities|AnyKey)
        (Default|ChangeHUD (Variables|Default|GetHUDMain) "NewEnumerator0")))))

(fn ConstructionScript)

(fn GetControllerID
  (bind _returnvalue (Class|GameplayStatics|GetPlayerControllerID (Variables|Default|GetController)))
  (return _returnvalue))