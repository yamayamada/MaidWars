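; Game instance for the maid game that tracks player-controlled BP_Owner characters and moves them to spawn points.
; SetPlayer fills the Player array in controller index order for up to four players, exposed through GetPlayer.
; SetAllSpawnPoint teleports each player-controlled owner to the BP_SpawnPoint matching the given mode and controller ID.
; SetIsGameStart is a stub that loops over players without effect, awaiting a flag.
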(fn SetPlayer
  ;[1 1 1] PlayerController０番目から順に配列にAddする
  (bind _outactors (Actor|GetAllActorsOfClass "/Game/Character/BP_Owner.BP_Owner_C"))
  (for _index (range 0 3)
    (for _array_element _outactors
      (if (== (Pawn|GetController _array_element) (Game|GetPlayerController _index))
        (Utilities|Array|Add (Variables|Default|GetPlayer) _array_element)))))

(fn GetPlayer
  (return (Variables|Default|GetPlayer)))

(fn SetIsGameStart
  (params (flg :type Boolean))
  ;[1 1 1] Flg作成後記入
  (for _array_element (Variables|Default|GetPlayer)
    _))

(fn SetAllSpawnPoint
  (params (Mode :type E_SpawnMode%20Enum :default "NewEnumerator0"))
  (bind _outactors (Actor|GetAllActorsOfClass "/Game/Character/BP_Owner.BP_Owner_C"))
  (for _array_element _outactors
    (bind _asplayer_controller (Utilities|Casting|CastToPlayerController (Pawn|GetController _array_element)))
    (Transformation|SetActorLocation _array_element (CallFunction|GetSpawnPoint Mode _asplayer_controller) false false)))

(fn GetSpawnPoint
  (params (Mode :type E_SpawnMode%20Enum :default "NewEnumerator0") (Controller :type Player%20Controller%20Object%20Reference))
  (bind _outactors (Actor|GetAllActorsOfClass "/Game/Map/MapData/BP_SpawnPoint.BP_SpawnPoint_C"))
  (for _array_element _outactors
    (bind _returnvalue (Class|GameplayStatics|GetPlayerControllerID Controller))
    (if (and (Utilities|Enum|Equal(Enum) Mode (Variables|/Game/Map/MapData/BP_SpawnPoint.BP_SpawnPoint_C|GetSpawnMode _array_element)) (== _returnvalue (Variables|/Game/Map/MapData/BP_SpawnPoint.BP_SpawnPoint_C|GetPlayerControllerNumber _array_element)))
      (return (Transformation|GetActorLocation _array_element)))))