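; BP_LaserChild is a laser weapon actor that flies forward as a shrinking sphere and destroys itself.
; BeginPlay scales the Sphere component uniformly from the Size variable.
; Each Tick moves the actor along its local X without sweep, decrements and reapplies Size, and destroys the actor once Size reaches zero.
; Movement and lifetime are frame-rate dependent because neither step uses delta time.
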(event EventBeginPlay
  (bind _size (Variables|Default|GetSize))
  (Transformation|SetWorldScale3D (Variables|Default|GetSphere) (Math|Vector|MakeVector _size _size _size)))

(event Collision|EventActorBeginOverlap
  (params (OtherActor :type Actor%20Object%20Reference)))

(event EventTick
  (params (DeltaSeconds :type Float%20%28single-precision%29))
  (Transformation|AddActorLocalOffset "25.000000, 0, 0" false false)
  (bind _output_get (Variables|Default|SetSize (- (Variables|Default|GetSize) 0.01)))
  (if (<= _output_get 0.0)
    (Actor|DestroyActor)
    (else
      (Transformation|SetWorldScale3D (Variables|Default|GetSphere) (Math|Vector|MakeVector (Variables|Default|GetSize) (Variables|Default|GetSize) (Variables|Default|GetSize))))))

(fn ConstructionScript)